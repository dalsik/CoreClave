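; Game mode for CoreClave, a turn-based two-player card game, handling player setup, turns and action points.
; PostLogin numbers each controller and sets its move direction.
; Server_RequestPassTurn validates the active player, flips the GameState turn index, banks unused AP in PlayerState and has the opponent's controller add a card.
; Server_Reroll allows one AP roll per turn through MyActionPointManager, factoring in stored AP and saving results to PlayerState.
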(event `self.ReceiveBeginPlay`
  ; 캐싱
  (bind _asgs_core_clave (cast `/Game/CoreClave/Assets/GameModeFiles/GS_CoreClave` (`GameplayStatics.GetGameState`)))
  (set `self.As GS Core Clave` _asgs_core_clave)
  (bind _returnvalue (`GameplayStatics.GetActorOfClass` "/Game/CoreClave/Assets/MyActionPointManager.MyActionPointManager_C"))
  (set `self.APManager` _returnvalue))

(event `self.K2_PostLogin`
  (params (NewPlayer :type "PlayerController Object Reference"))
  ; 사용자 접속 시, 고유의 플레이어 인덱스 할당
  (bind _asbp_core_clave_player_controller (cast `/Game/CoreClave/Assets/GameModeFiles/BP_CoreClavePlayerController` NewPlayer))
  (set `/Game/CoreClave/Assets/GameModeFiles/BP_CoreClavePlayerController.MyPlayer_idx` (`self.PlayerCount`) _asbp_core_clave_player_controller)
  (bind _output_get (set `self.PlayerCount` (+ (`self.PlayerCount`) 1)))
  (`KismetSystemLibrary.PrintString` (`KismetStringLibrary.Conv_IntToString` _output_get))
  (if (== (`/Game/CoreClave/Assets/GameModeFiles/BP_CoreClavePlayerController.MyPlayer_idx` _asbp_core_clave_player_controller) 1)
    (set `/Game/CoreClave/Assets/GameModeFiles/BP_CoreClavePlayerController.Player_MoveDirection` 1 _asbp_core_clave_player_controller)
    (else
      (set `/Game/CoreClave/Assets/GameModeFiles/BP_CoreClavePlayerController.Player_MoveDirection` -1 _asbp_core_clave_player_controller))))

(event `Server_RequestPassTurn`
  (params (PlayerIdx :type Integer) (PlayerController :type "/Game/CoreClave/Assets/GameModeFiles/BP_CoreClavePlayerController Object Reference"))
  (bind _as_gs_core_clave (`self.As GS Core Clave`))
  (bind _currentturnplayer_idx (`/Game/CoreClave/Assets/GameModeFiles/GS_CoreClave.CurrentTurnPlayer_Idx` _as_gs_core_clave))
  (if (== (`/Game/CoreClave/Assets/GameModeFiles/GS_CoreClave.CurrentTurnPlayer_Idx` (`self.As GS Core Clave`)) PlayerIdx)
    ; 현재 GameState의 플레이어 idx가 0일경우에 버튼을 누르면 + 1을, 1이면 0으로 설정
    (if (== _currentturnplayer_idx 0)
      (set `/Game/CoreClave/Assets/GameModeFiles/GS_CoreClave.CurrentTurnPlayer_Idx` (+ _currentturnplayer_idx 1) _as_gs_core_clave)
      (else
        (set `/Game/CoreClave/Assets/GameModeFiles/GS_CoreClave.CurrentTurnPlayer_Idx` (- _currentturnplayer_idx 1) _as_gs_core_clave)))
    ; 턴 넘길 때 현재 사용하지 않은 AP를 다음 AP에 추가할 수 있도록 해야한다
    (bind _asps_core_clave (cast `/Game/CoreClave/Assets/GameModeFiles/PS_CoreClave` (`Controller.PlayerState` PlayerController)))
    (bind (_outstoredactionpoints _outremainingactionpoints) (`ActionPointManager.BankRemainingActionPoints` (`self.APManager`) (`/Game/CoreClave/Assets/GameModeFiles/PS_CoreClave.CurrentAP` _asps_core_clave)))
    (`/Game/CoreClave/Assets/GameModeFiles/PS_CoreClave.SetStoredAP` _asps_core_clave _outstoredactionpoints _outremainingactionpoints)
    (`/Game/CoreClave/Assets/GameModeFiles/PS_CoreClave.OnStoredAPChanged` _asps_core_clave _outstoredactionpoints)
    (set `/Game/CoreClave/Assets/GameModeFiles/PS_CoreClave.bHasRolledThisTurn` false _asps_core_clave)
    ; 자신의 인덱스를 활용해서 자신의 카드를 추가하는 것이 아니라, 버튼을 눌렀을 때, 상대방의 카드가 늘어나도록
    (if (== PlayerIdx 0)
      (bind _output_get (set `self.Card_Add_idx` 1))
      (bind _asbp_core_clave_player_controller (cast `/Game/CoreClave/Assets/GameModeFiles/BP_CoreClavePlayerController` (`GameplayStatics.GetPlayerController` _output_get)))
      (`/Game/CoreClave/Assets/GameModeFiles/BP_CoreClavePlayerController.ClientRPC_AddCard` _asbp_core_clave_player_controller)
      (else
        (bind _output_get_2 (set `self.Card_Add_idx` 0))
        (bind _asbp_core_clave_player_controller_2 (cast `/Game/CoreClave/Assets/GameModeFiles/BP_CoreClavePlayerController` (`GameplayStatics.GetPlayerController` _output_get_2)))
        (bind _output_get_3 (set `self.As BP Core Clave Player Controller` _asbp_core_clave_player_controller_2))
        (`/Game/CoreClave/Assets/GameModeFiles/BP_CoreClavePlayerController.ClientRPC_AddCard` _output_get_3)))))

(event `Server_Reroll`
  (params (PlayerController :type "/Game/CoreClave/Assets/GameModeFiles/BP_CoreClavePlayerController Object Reference"))
  ; AP포인트 설정 로직
  (bind _asps_core_clave (cast `/Game/CoreClave/Assets/GameModeFiles/PS_CoreClave` (`Controller.PlayerState` PlayerController)))
  (if (not (`/Game/CoreClave/Assets/GameModeFiles/PS_CoreClave.bHasRolledThisTurn` _asps_core_clave))
    (bind (_outcurrentactionpoints _outstoredactionpoints _outlastrollresult) (`ActionPointManager.RollActionPoints` (`self.APManager`) (`/Game/CoreClave/Assets/GameModeFiles/PS_CoreClave.StoredAP` _asps_core_clave)))
    (bind _output_get (set `/Game/CoreClave/Assets/GameModeFiles/PS_CoreClave.CurrentAP` _outcurrentactionpoints _asps_core_clave))
    (bind _output_get_2 (set `/Game/CoreClave/Assets/GameModeFiles/PS_CoreClave.StoredAP` _outstoredactionpoints _asps_core_clave))
    (bind _output_get_3 (set `/Game/CoreClave/Assets/GameModeFiles/PS_CoreClave.LastRollResult` _outlastrollresult _asps_core_clave))
    (set `/Game/CoreClave/Assets/GameModeFiles/PS_CoreClave.bHasRolledThisTurn` true _asps_core_clave)
    (`KismetSystemLibrary.PrintText` (`|FormatText` "현재 AP ! : {0}" (`KismetTextLibrary.Conv_IntToText` _output_get)))
    (`KismetSystemLibrary.PrintText` (`|FormatText` "저장된 AP! : {0}" (`KismetTextLibrary.Conv_IntToText` _output_get_2)))
    (`KismetSystemLibrary.PrintText` (`|FormatText` "리롤 돌린 결과 ! : {0}" (`KismetTextLibrary.Conv_IntToText` _output_get_3)))))

(fn `UserConstructionScript`)