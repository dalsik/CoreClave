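; Player controller for a two-player networked card game that gives each player their own camera and spawns their units.
; When the replicated player index arrives, SetupCamera switches the local controller to the CameraActor tagged Player1 or Player2 and opens CardUI with game-and-UI input.
; Server_SpawnUnit spawns Card1 at the requested location, yawed to face by player index, ignoring its SpawnClass argument.
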(event `self.ReceiveBeginPlay`)

(event `Server_SpawnUnit`
  (params (SpawnClass :type "SkeletalMesh Object Reference") (SpawnLocation :type "Vector Structure"))
  (switch `int` (`self.MyPlayer_idx`)
    (:`0`
      (`|SpawnActorFromClass` "/Game/CoreClave/Assets/Card1.Card1_C" (`KismetMathLibrary.MakeTransform` SpawnLocation (struct :`Yaw` -90.0)) "AlwaysSpawn" "MultiplyWithRoot" self null)
      (`KismetSystemLibrary.PrintString` "0번 인덱스 플레이어 병사 스폰!"))
    (:`1`
      (`|SpawnActorFromClass` "/Game/CoreClave/Assets/Card1.Card1_C" (`KismetMathLibrary.MakeTransform` SpawnLocation (struct :`Yaw` 90.0)) "AlwaysSpawn" "MultiplyWithRoot" self null)
      (`KismetSystemLibrary.PrintString` "1번 인덱스 플레이어 병사 스폰!"))))

(fn `OnRep_MyPlayer_idx`
  (`self.SetupCamera`)
  (`KismetSystemLibrary.PrintString` "OnRep 실행됨"))

(fn `SetupCamera`
  (if (`self.IsLocalController`)
    (switch `int` (`self.MyPlayer_idx`)
      (:`0`
        (bind _outactors (`GameplayStatics.GetAllActorsOfClassWithTag` "/Script/Engine.CameraActor" "Player1"))
        (`self.SetViewTargetWithBlend` self (`|GetArrayItem` _outactors) 0.0 "VTBlend_Linear" 20.0 false)
        (`KismetSystemLibrary.PrintString` "00000000000000")
        (bind _returnvalue (`|CreateWidget` "/Game/CoreClave/Assets/UI/CardUI.CardUI_C" self))
        (`UserWidget.AddToViewport` _returnvalue 0)
        (`WidgetBlueprintLibrary.SetInputMode_GameAndUIEx` self _returnvalue "DoNotLock" false))
      (:`1`
        (bind _outactors_2 (`GameplayStatics.GetAllActorsOfClassWithTag` "/Script/Engine.CameraActor" "Player2"))
        (`self.SetViewTargetWithBlend` self (`|GetArrayItem` _outactors_2) 0.0 "VTBlend_Linear" 20.0 false)
        (`KismetSystemLibrary.PrintString` "111111111111")
        (bind _returnvalue_2 (`|CreateWidget` "/Game/CoreClave/Assets/UI/CardUI.CardUI_C" self))
        (bind _output_get (set `self.NewVar` _returnvalue_2))
        (`UserWidget.AddToViewport` _output_get 0)
        (`WidgetBlueprintLibrary.SetInputMode_GameAndUIEx` self _returnvalue_2 "DoNotLock" false)))
    (else
      (`KismetSystemLibrary.PrintString` "로컬 플레이어 아님!"))))

(fn `UserConstructionScript`)