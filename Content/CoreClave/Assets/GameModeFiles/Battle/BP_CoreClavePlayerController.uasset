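; Player controller for the two-player CoreClave card battle, handling each player's camera, card UI, unit placement and movement on the grid.
; Replicated player index picks the tagged camera and creates the card widget; dragging a card slides the camera and line-traces cells for highlights and unit previews.
; Spawning checks mana against the card table, and clicks move own units within reachable cells, spending AP.
; Passing and rerolls go through the game mode.
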(event `CardDragOver_Delegate`
  (bind _mycardui (`self.MyCardUI`))
  (bind _wbp_description (`/Game/CoreClave/Assets/UI/CardUI.WBP_Description` _mycardui))
  (bind _gradient (`/Game/CoreClave/Assets/UI/CardUI.Gradient` _mycardui))
  ; 카드 드래그 시 Gradient UI  표시, 카드 드래그 안하면 해제
  (if (`self.IsCardDragging`)
    (`/Game/CoreClave/Assets/UI/Gradient.OnGradient` _gradient)
    (`/Game/CoreClave/Assets/UI/WBP_Description.On Description` _wbp_description)
    ; 0이면 클라0, 아니면 클라1
    (if (== (`self.MyPlayer_idx`) 0)
      (bind (_direction `_새_트랙_0`) (`Timeline|타임라인` :!via `PlayFromStart`)
        (:`Update`
          (`self.K2_SetActorLocation` (`self.Camaer(Player1)`) (`KismetMathLibrary.VLerp` (`self.Camera1_Pos`) (`self.Camera1_TargetPos`) `_새_트랙_0`) false false)))
      (else
        (bind (_direction_2 `_새_트랙_0_2`) (`Timeline|타임라인_0` :!via `PlayFromStart`)
          (:`Update`
            (`self.K2_SetActorLocation` (`self.Camera(Player2)`) (`KismetMathLibrary.VLerp` (`self.Camera2_Pos`) (`self.Camera2_TargetPos`) `_새_트랙_0_2`) false false)))))
    (else
      (`/Game/CoreClave/Assets/UI/Gradient.OffGradient` _gradient)
      (`/Game/CoreClave/Assets/UI/WBP_Description.Off Description` _wbp_description)
      ; 0이면 클라0, 아니면 클라1
      (if (== (`self.MyPlayer_idx`) 0)
        (bind (_direction_3 `_새_트랙_0_3`) (`Timeline|타임라인_1` :!via `PlayFromStart`)
          (:`Update`
            (`self.K2_SetActorLocation` (`self.Camaer(Player1)`) (`KismetMathLibrary.VLerp` (`self.Camera1_TargetPos`) (`self.Camera1_Pos`) `_새_트랙_0_3`) false false)))
        (else
          (bind (_direction_4 `_새_트랙_0_4`) (`Timeline|타임라인_2` :!via `PlayFromStart`)
            (:`Update`
              (`self.K2_SetActorLocation` (`self.Camera(Player2)`) (`KismetMathLibrary.VLerp` (`self.Camera2_TargetPos`) (`self.Camera2_Pos`) `_새_트랙_0_4`) false false))))))))

(event `self.ReceiveBeginPlay`
  (bind _returnvalue (`KismetMathLibrary.Conv_VectorToTransform` (0.0 0.0 -100.0)))
  (bind _returnvalue_2 (`KismetMathLibrary.Conv_VectorToTransform` (0.0 0.0 -100.0)))
  (bind _player_movedirection (`self.Player_MoveDirection`))
  (bind _player_movedirection_2 (`self.Player_MoveDirection`))
  (bind _asgs_core_clave (cast `/Game/CoreClave/Assets/GameModeFiles/Battle/GS_CoreClave` (`GameplayStatics.GetGameState`)))
  (set `self.As GS Core Clave` _asgs_core_clave)
  (bind _returnvalue_3 (`GameplayStatics.GetActorOfClass` "/Game/CoreClave/Assets/BP_GridManager.BP_GridManager_C"))
  (set `self.GridManager` _returnvalue_3)
  (bind _output_get (set `self.Player State` (`self.PlayerState`)))
  (`/Engine/EditorBlueprintResources/StandardMacros.IsValid` _output_get
    (:`Is Valid`
      (bind _asps_core_clave (cast `/Game/CoreClave/Assets/GameModeFiles/Battle/PS_CoreClave` (stale `TrygetPs` _output_get) :!label _label)
        (:`then`
          (set `self.As PS Core Clave` _asps_core_clave)
          (if (`self.IsLocalPlayerController`)
            (bind _returnvalue_4 (`|SpawnActorFromClass` "/Game/CoreClave/Assets/LineFeedback_self.LineFeedback_self_C" _returnvalue "Undefined" "MultiplyWithRoot" null null))
            (`/Game/CoreClave/Assets/LineFeedback_self.SetMoveDirection` _returnvalue_4 _player_movedirection_2)
            (bind _returnvalue_5 (`|SpawnActorFromClass` "/Game/CoreClave/Assets/LineFeedback_other.LineFeedback_other_C" _returnvalue "Undefined" "MultiplyWithRoot" null null))
            (`/Game/CoreClave/Assets/LineFeedback_other.SetMoveDirection` _returnvalue_5 (* _player_movedirection_2 -1))
            (bind _returnvalue_6 (`|SpawnActorFromClass` "/Game/CoreClave/Assets/LineFeedback_Side_self.LineFeedback_Side_self_C" _returnvalue_2 "Undefined" "MultiplyWithRoot" null null))
            (`/Game/CoreClave/Assets/LineFeedback_Side_self.SetMoveDirection_Side` _returnvalue_6 _player_movedirection)
            (bind _returnvalue_7 (`|SpawnActorFromClass` "/Game/CoreClave/Assets/LineFeedback_Side_other.LineFeedback_Side_other_C" _returnvalue_2 "Undefined" "MultiplyWithRoot" null null))
            (`/Game/CoreClave/Assets/LineFeedback_Side_other.SetMoveDirection_Side` _returnvalue_7 (* _player_movedirection -1)))
          ; 이거는 서버역할을 하는 클라이언트0에만 GM변수가 생성됨
          (bind _asgm_core_clave (cast `/Game/CoreClave/Assets/GameModeFiles/Battle/GM_CoreClave` (`GameplayStatics.GetGameMode`)))
          (set `self.As GM Core Clave` _asgm_core_clave))
        (:`CastFailed`
          (`KismetSystemLibrary.K2_SetTimerDelegate` (delegate `TrygetPs`) 0.2 :!label _label_2))))
    (:`Is Not Valid`
      (goto _label_2))))

(event `TrygetPs`
  (bind _output_get (set `self.Player State` (`self.PlayerState`)))
  (`/Engine/EditorBlueprintResources/StandardMacros.IsValid` _output_get
    (:`Is Valid`
      (goto _label))
    (:`Is Not Valid`
      (goto _label_2))))

(event `self.ReceiveTick`
  (params (DeltaSeconds :type "Float (single-precision)"))
  (bind _gridmanager (`self.GridManager`))
  (bind (_worldposition _worlddirection) (`GameplayStatics.DeprojectScreenToWorld` self (`self.CachedMousePosition`)))
  ; 드래그 감지 시 계속 라인트레이스 쏘는 로직
  (if (`self.IsCardDragging`)
    (bind _outhit (`KismetSystemLibrary.LineTraceSingle` _worldposition (+ _worldposition (* _worlddirection 10000.0)) "TraceTypeQuery1"))
    (bind _asbp_grid_cell (cast `/Game/CoreClave/Assets/BP_GridCell` (`.HitActor` (`GameplayStatics.BreakHitResult` _outhit)))
      (:`then`
        (`/Engine/EditorBlueprintResources/StandardMacros.IsValid` _asbp_grid_cell
          (:`Is Valid`
            (`/Engine/EditorBlueprintResources/StandardMacros.IsValid` _gridmanager
              (:`Is Valid`
                (`GridManager.UpdateDragHighlight` _gridmanager _asbp_grid_cell (`self.Player_MoveDirection`))
                (`GridManager.UpdateUnitPreview` _gridmanager _asbp_grid_cell (`self.PreviewUnitClass`) (`self.CurrentCardID`) (`self.Player_MoveDirection`))
                (if (not (== (`.HitActor` (`GameplayStatics.BreakHitResult` _outhit)) (`self.LastHoveredCell`)))
                  (if (`GridManager.IsPlaceableCell` (`self.GridManager`) (`GridCell.Row` _asbp_grid_cell) (`GridCell.Col` _asbp_grid_cell) (`self.Player_MoveDirection`))
                    (`GameplayStatics.PlaySound2D` "/Game/CoreClave/mp3/GridCellButton.GridCellButton" 1.0 1.0 0.0 null null))
                  (set `self.LastHoveredCell` _asbp_grid_cell)))))))
      (:`CastFailed`
        (`GridManager.ClearAllHighlights` _gridmanager)
        (`GridManager.ClearUnitPreview` _gridmanager)))))

(event `ClientRPC_AddCard_Req`
  (bind _gridmanager (`self.GridManager`))
  (bind _as_gs_core_clave (`self.As GS Core Clave`))
  ; 버튼이 눌렸을 때, 서버에게 GM에 있는 함수(차례 인덱스 변경해주는) 실행해달라고 함
  (if (not (`/Game/CoreClave/Assets/GameModeFiles/Battle/PS_CoreClave.bHasPassButton` (`self.As PS Core Clave`)))
    (set `/Game/CoreClave/Assets/GameModeFiles/Battle/PS_CoreClave.bHasPassButton` true (`self.As PS Core Clave`))
    (`/Game/CoreClave/Assets/GameModeFiles/Battle/GM_CoreClave.Server_RequestPassTurn` (`self.As GM Core Clave`) (`self.MyPlayer_idx`) self)
    ; 현재 플레이어 컨트롤러의 MoveDirection이 1일 경우 send -1
    (if (== (`self.Player_MoveDirection`) 1)
      (`GridManager.AdvanceAllUnits` _gridmanager -1)
      (else
        (`GridManager.AdvanceAllUnits` _gridmanager 1)))
    ; 현재 턴수 증가
    (bind _output_get (set `/Game/CoreClave/Assets/GameModeFiles/Battle/GS_CoreClave.CurrentTurn` (+ (`/Game/CoreClave/Assets/GameModeFiles/Battle/GS_CoreClave.CurrentTurn` _as_gs_core_clave) 1) _as_gs_core_clave))
    (`KismetSystemLibrary.PrintString` (`KismetTextLibrary.Conv_TextToString` (`|FormatText` "현재턴수{0}" _output_get)))
    (for _array_element (`GameStateBase.PlayerArray` _as_gs_core_clave)
      (bind _asps_core_clave (cast `/Game/CoreClave/Assets/GameModeFiles/Battle/PS_CoreClave` _array_element))
      (set `/Game/CoreClave/Assets/GameModeFiles/Battle/PS_CoreClave.CurrentMana` _output_get _asps_core_clave))))

(event `ClientRPC_AddCard`
  ; GM의 함수가 끝나면 이 함수가 호출되어 카드가 추가됨
  (`CoreClaveUserWidget.AddCardTohand` (`self.MyCardUI`)))

(event `Server_SpawnUnit`
  (params (SpawnLocation :type "Vector Structure") (Col :type Integer) (Row :type Integer) (CardId :type Name))
  (bind _gridmanager (`self.GridManager`))
  (bind _player_movedirection (`self.Player_MoveDirection`))
  (bind _as_ps_core_clave (`self.As PS Core Clave`))
  ; 로컬 컨트롤러 플레이어의 인덱스를 기반으로 스폰하고자 하는 유닛을 스 폰
  (`KismetSystemLibrary.PrintString` (`KismetStringLibrary.Conv_IntToString` Col))
  (`KismetSystemLibrary.PrintString` (`KismetStringLibrary.Conv_IntToString` Row))
  (`KismetSystemLibrary.PrintString` "스폰 호출됨")
  (bind _returnvalue (`|GetDataTableRow` "/Game/CoreClave/Assets/CoreClave_DT.CoreClave_DT" CardId)
    (:`then`
      (switch `int` (`self.MyPlayer_idx`)
        (:`0`
          (bind _canspawn (`/Game/CoreClave/Assets/GameModeFiles/Battle/PS_CoreClave.CompareMana` _as_ps_core_clave (`.Cost` (break `CardStatData` _returnvalue))))
          (if _canspawn
            (bind _returnvalue_2 (`GridManager.SpawnUnitAtCell` _gridmanager Row Col "/Game/CoreClave/Assets/Card_normal_0.Card_normal_0_C" _player_movedirection))
            (if (`KismetSystemLibrary.IsValid` _returnvalue_2)
              (`self.K2_SetActorRotation` _returnvalue_2 (struct :`Yaw` -90.0) false)
              (bind _ascard_unit_actor (cast `CardUnitActor` _returnvalue_2))
              (`CardUnitActor.InitializeUnit` _ascard_unit_actor CardId)
              (`KismetSystemLibrary.PrintString` "0번 인덱스 플레이어 병사 스폰!")
              (`self.SendClearCardUI` :!label _label_3))
            (else
              (`self.SendClearHighlight/Preview` :!label _label_4))))
        (:`1`
          (bind _canspawn_2 (`/Game/CoreClave/Assets/GameModeFiles/Battle/PS_CoreClave.CompareMana` _as_ps_core_clave (`.Cost` (break `CardStatData` _returnvalue))))
          (if _canspawn_2
            (bind _returnvalue_3 (`GridManager.SpawnUnitAtCell` _gridmanager Row Col "/Game/CoreClave/Assets/Card_normal_0.Card_normal_0_C" _player_movedirection))
            (if (`KismetSystemLibrary.IsValid` _returnvalue_3)
              (`self.K2_SetActorRotation` _returnvalue_3 (struct :`Yaw` 90.0) false)
              (bind _ascard_unit_actor_2 (cast `CardUnitActor` _returnvalue_3))
              (`CardUnitActor.InitializeUnit` _ascard_unit_actor_2 CardId)
              (`KismetSystemLibrary.PrintString` "1번 인덱스 플레이어 병사 스폰!")
              (goto _label_3))
            (else
              (goto _label_4))))))))

(event `ReRoll`
  ; 서버(GM)에서 AP 포인트 변경하도록 호출
  (`/Game/CoreClave/Assets/GameModeFiles/Battle/GM_CoreClave.Server_Reroll` (`self.As GM Core Clave`) self))

(event `SendClearCardUI`
  ; 대신 서버에서 실행으로 설정된 Spaw함수에서 실행되는 거니까 소유중인 클라이언트에서 실행으로 설정
  ;; 스폰 성공 시에는 ClearCardUI / 스폰 실패 시에는 Clear Highlihgt/Preview
  (`/Game/CoreClave/Assets/UI/CardUI.ClearCardUI` (`self.MyCardUI`)))

(event `SendClearHighlight/Preview`
  ; 대신 서버에서 실행으로 설정된 Spaw함수에서 실행되는 거니까 소유중인 클라이언트에서 실행으로 설정
  ;; 스폰 성공 시에는 ClearCardUI / 스폰 실패 시에는 Clear Highlihgt/Preview
  (`/Game/CoreClave/Assets/UI/CardUI.ClearHighlight/Preview` (`self.MyCardUI`)))

(event `Owning_SetProgress`
  (`self.SetManaProgress`))

(event `Owning_ManaText`
  (params (Cost :type Integer))
  (if (not (`self.HasAuthority`))
    (`self.SetManaText(Spawn)` Cost)))

(event `EnhancedInput|/Game/CoreClave/Input/IA_Click`
  (params (ActionValue :type Boolean) (ElapsedSeconds :type "Float (double-precision)") (TriggeredSeconds :type "Float (double-precision)") (InputAction :type "InputAction Object Reference" :default "/Game/CoreClave/Input/IA_Click.IA_Click"))
  ; 클릭시
  (:`Triggered`
    (`self.HandleLeftClick`)))

(event `HandleLeftClick`
  (bind _hitresult (`self.GetHitResultUnderCursorByChannel` "TraceTypeQuery4"))
  (bind _gridmanager (`self.GridManager`))
  (bind _gridmanager_2 (`self.GridManager`))
  (bind _selectedcell (`self.SelectedCell`))
  (if (== (`/Game/CoreClave/Assets/GameModeFiles/Battle/GS_CoreClave.CurrentTurnPlayer_Idx` (`self.As GS Core Clave`)) (`self.MyPlayer_idx`))
    (if (`GameplayStatics.BreakHitResult` _hitresult)
      (bind _asbp_grid_cell (cast `/Game/CoreClave/Assets/BP_GridCell` (`.HitActor` (`GameplayStatics.BreakHitResult` _hitresult))))
      (bind _ascard_unit_actor (cast `CardUnitActor` (`GridCell.OccupyingUnit` _asbp_grid_cell))
        (:`then`
          (if (== (`self.Player_MoveDirection`) (`CardUnitActor.MoveDirection` _ascard_unit_actor))
            (bind _output_get (set `self.SelectedCell` _asbp_grid_cell))
            ; 하이라이트 설정 후, ReachableCell 변수에 할당
            (`GridManager.ClearReachableHighlights` _gridmanager)
            (bind _returnvalue (`GridManager.GetReachableCells` _gridmanager _output_get (`/Game/CoreClave/Assets/GameModeFiles/Battle/PS_CoreClave.CurrentAP` (`self.As PS Core Clave`))))
            (set `self.ReachableCells` _returnvalue)
            (`GridManager.HighlightReachableCells` _gridmanager _returnvalue)
            (else
              ; 만약 점유되고 있는 유닛이 없는 경우이면서,
              (if (`KismetArrayLibrary.Array_Contains` (`self.ReachableCells`) _asbp_grid_cell) :!label _label_5
                (`self.MoveUnit` (`GridCell.Row` _selectedcell) (`GridCell.Col` _selectedcell) (`GridCell.Row` _asbp_grid_cell) (`GridCell.Col` _asbp_grid_cell))
                (`GridManager.UpdateFrontlineCache` _gridmanager_2)
                (`GridManager.ClearReachableHighlights` _gridmanager_2)
                (else
                  ;; 하이라이트가 아닌 셀을 클릭할 경우 하이라이트를 제거
                  (`GridManager.ClearReachableHighlights` (`self.GridManager`)))))))
        (:`CastFailed`
          (goto _label_5)))
      (else
        (`GridManager.ClearReachableHighlights` (`self.GridManager`))))))

(event `MoveUnit`
  (params (SelectedRow :type Integer) (SelectedCol :type Integer) (ClickedRow :type Integer) (ClickedCol :type Integer))
  (bind _as_ps_core_clave (`self.As PS Core Clave`))
  (bind _gridmanager (`self.GridManager`))
  (`KismetSystemLibrary.PrintText` (`|FormatText` "Selected Cell Row : {0}, Col {1};" SelectedRow SelectedCol))
  (`KismetSystemLibrary.PrintText` (`|FormatText` "Clicked Cell Row : {0}, Col {1};" ClickedRow ClickedCol))
  ; 만약 하이라이트 된 셀을 클릭할 경우 해당 셀로 이동
  (bind _returnvalue (`GridManager.MoveUnit` (`self.GridManager`) SelectedRow SelectedCol ClickedRow ClickedCol))
  (if _returnvalue
    (set `/Game/CoreClave/Assets/GameModeFiles/Battle/PS_CoreClave.CurrentAP` (- (`/Game/CoreClave/Assets/GameModeFiles/Battle/PS_CoreClave.CurrentAP` _as_ps_core_clave) (`KismetMathLibrary.Abs_Int` (+ (- SelectedRow ClickedRow) (- SelectedCol ClickedCol)))) _as_ps_core_clave)
    (`GridManager.ClearReachableHighlights` _gridmanager)
    (`GridManager.UpdateFrontlineCache` _gridmanager)))

(fn `OnRep_MyPlayer_idx`
  (`self.SetupCamera`)
  (`KismetSystemLibrary.PrintString` "OnRep 실행됨")
  (`KismetSystemLibrary.PrintText` (`|FormatText` "현재 CardUI{)}" (`KismetTextLibrary.Conv_ObjectToText` (`self.MyCardUI`)))))

(fn `OnRep_Player State`
  (bind _mycardui (`self.MyCardUI`))
  (`/Engine/EditorBlueprintResources/StandardMacros.IsValid` (`self.Player State`)
    (:`Is Valid`
      (`/Engine/EditorBlueprintResources/StandardMacros.IsValid` _mycardui
        (:`Is Valid`
          (`/Game/CoreClave/Assets/UI/CardUI.Initialize PS&Mana&Progress` _mycardui self)
          (return))))))

(fn `SetManaProgress`
  (bind _mycardui (`self.MyCardUI`))
  (if (== (`/Game/CoreClave/Assets/GameModeFiles/Battle/GS_CoreClave.CurrentTurnPlayer_Idx` (`self.As GS Core Clave`)) (`self.MyPlayer_idx`))
    (`/Engine/EditorBlueprintResources/StandardMacros.IsValid` _mycardui
      (:`Is Valid`
        (`/Game/CoreClave/Assets/UI/WBP_ManaProgress.VisualUpdateProgress` (`/Game/CoreClave/Assets/UI/WBP_Mana.WBP_ManaProgress` (`/Game/CoreClave/Assets/UI/CardUI.WBP_Mana` _mycardui)) (+ (`/Game/CoreClave/Assets/GameModeFiles/Battle/GS_CoreClave.CurrentTurn` (`self.As GS Core Clave`)) 1))))))

(fn `SetManaText`
  (if (== (`/Game/CoreClave/Assets/GameModeFiles/Battle/GS_CoreClave.CurrentTurnPlayer_Idx` (`self.As GS Core Clave`)) (`self.MyPlayer_idx`))
    (`/Game/CoreClave/Assets/UI/WBP_Mana_Text.Visual_SetText` (`/Game/CoreClave/Assets/UI/CardUI.WBP_Mana_Text` (`self.MyCardUI`)) (+ (`/Game/CoreClave/Assets/GameModeFiles/Battle/GS_CoreClave.CurrentTurn` (`self.As GS Core Clave`)) 1))))

(fn `SetManaText(Spawn)`
  (params (UnitCost :type Integer))
  (`/Game/CoreClave/Assets/UI/WBP_Mana_Text.Visual_SetText` (`/Game/CoreClave/Assets/UI/CardUI.WBP_Mana_Text` (`self.MyCardUI`)) (- (`/Game/CoreClave/Assets/GameModeFiles/Battle/PS_CoreClave.CurrentMana` (`self.As PS Core Clave`)) UnitCost)))

(fn `SetupCamera`
  (if (`self.IsLocalController`)
    (switch `int` (`self.MyPlayer_idx`)
      (:`0`
        (bind _outactors (`GameplayStatics.GetAllActorsOfClassWithTag` "/Script/Engine.CameraActor" "Player1"))
        (bind _output_get (set `self.Camaer(Player1)` (`|GetArrayItem` _outactors)))
        (bind _output_get_2 (set `self.Camera1_Pos` (-650.0 0.0 1000.0)))
        (set `self.Camera1_TargetPos` (+ _output_get_2 (0.0 -200.0 0.0)))
        (`self.SetViewTargetWithBlend` self _output_get 0.0 "VTBlend_Linear" 20.0 false))
      (:`1`
        (bind _outactors_2 (`GameplayStatics.GetAllActorsOfClassWithTag` "/Script/Engine.CameraActor" "Player2"))
        (bind _output_get_3 (set `self.Camera(Player2)` (`|GetArrayItem` _outactors_2)))
        (bind _output_get_4 (set `self.Camera2_Pos` (650.0 0.0 1000.0)))
        (set `self.Camera2_TargetPos` (+ _output_get_4 (0.0 200.0 0.0)))
        (`self.SetViewTargetWithBlend` self _output_get_3 0.0 "VTBlend_Linear" 20.0 false)))
    (bind _returnvalue (`|CreateWidget` "/Game/CoreClave/Assets/UI/CardUI.CardUI_C" self))
    (bind _output_get_5 (set `self.MyCardUI` _returnvalue))
    (`UserWidget.AddToViewport` _output_get_5 0)
    (`WidgetBlueprintLibrary.SetInputMode_GameAndUIEx` self _returnvalue "DoNotLock" false)
    (else
      (`KismetSystemLibrary.PrintString` "로컬 플레이어 아님!"))))

(fn `UserConstructionScript`)