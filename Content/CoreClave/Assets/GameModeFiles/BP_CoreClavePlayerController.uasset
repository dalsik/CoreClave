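; Player controller for CoreClave's turn-based card game, where players place units on a grid.
; While a card is dragged, Tick traces under the cached cursor to drive GridManager highlights and unit previews.
; The replicated player index selects the tagged camera, creates the card UI and sets spawned units' facing.
; Pass and reroll requests go to GM_CoreClave; passing also advances units in the opposite move direction and increments the turn.
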(event `self.ReceiveTick`
  (params (DeltaSeconds :type "Float (single-precision)"))
  (bind _gridmanager (`self.GridManager`))
  (bind (_worldposition _worlddirection) (`GameplayStatics.DeprojectScreenToWorld` self (`self.CachedMousePosition`)))
  ; 드래그 감지 시 계속 라인트레이스 쏘는 로직
  (if (`self.IsCardDragging`)
    (bind _outhit (`KismetSystemLibrary.LineTraceSingle` _worldposition (+ _worldposition (* _worlddirection 10000.0)) "TraceTypeQuery1"))
    (bind _asbp_grid_cell (cast `/Game/CoreClave/Assets/BP_GridCell` (`.HitActor` (`GameplayStatics.BreakHitResult` _outhit)))
      (:`then`
        (`/Engine/EditorBlueprintResources/StandardMacros.IsValid` _asbp_grid_cell
          (:`Is Valid`
            (`/Engine/EditorBlueprintResources/StandardMacros.IsValid` _gridmanager
              (:`Is Valid`
                (`GridManager.UpdateDragHighlight` _gridmanager _asbp_grid_cell (`self.Player_MoveDirection`))
                (`GridManager.UpdateUnitPreview` _gridmanager _asbp_grid_cell (`self.PreviewUnitClass`) (`self.CurrentCardID`) (`self.Player_MoveDirection`))
                (if (not (== (`.HitActor` (`GameplayStatics.BreakHitResult` _outhit)) (`self.LastHoveredCell`)))
                  (if (`GridManager.IsPlaceableCell` (`self.GridManager`) (`GridCell.Row` _asbp_grid_cell) (`GridCell.Col` _asbp_grid_cell) (`self.Player_MoveDirection`))
                    (`GameplayStatics.PlaySound2D` "/Game/CoreClave/mp3/GridCellButton.GridCellButton" 1.0 1.0 0.0 null null))
                  (set `self.LastHoveredCell` _asbp_grid_cell)))))))
      (:`CastFailed`
        (`GridManager.ClearAllHighlights` _gridmanager)
        (`GridManager.ClearUnitPreview` _gridmanager)))))

(event `self.ReceiveBeginPlay`
  (bind _asgs_core_clave (cast `/Game/CoreClave/Assets/GameModeFiles/GS_CoreClave` (`GameplayStatics.GetGameState`)))
  (set `self.As GS Core Clave` _asgs_core_clave)
  (bind _returnvalue (`GameplayStatics.GetActorOfClass` "/Game/CoreClave/Assets/BP_GridManager.BP_GridManager_C"))
  (set `self.GridManager` _returnvalue)
  (bind _output_get (set `self.Player State` (`self.PlayerState`)))
  (bind _asgm_core_clave (cast `/Game/CoreClave/Assets/GameModeFiles/GM_CoreClave` (`GameplayStatics.GetGameMode`)))
  (set `self.As GM Core Clave` _asgm_core_clave)
  (bind _asps_core_clave (cast `/Game/CoreClave/Assets/GameModeFiles/PS_CoreClave` _output_get))
  (set `self.As PS Core Clave` _asps_core_clave))

(event `ClientRPC_AddCard`
  ; GM의 함수가 끝나면 이 함수가 호출되어 카드가 추가됨
  (`CoreClaveUserWidget.AddCardTohand` (`self.MyCardUI`)))

(event `ClientRPC_AddCard_Req`
  (bind _gridmanager (`self.GridManager`))
  (bind _as_gs_core_clave (`self.As GS Core Clave`))
  ; 버튼이 눌렸을 때, 서버에게 GM에 있는 함수(차례 인덱스 변경해주는) 실행해달라고 함
  (if (not (`/Game/CoreClave/Assets/GameModeFiles/PS_CoreClave.bHasPassButton` (`self.As PS Core Clave`)))
    (`/Game/CoreClave/Assets/GameModeFiles/GM_CoreClave.Server_RequestPassTurn` (`self.As GM Core Clave`) (`self.MyPlayer_idx`) self)
    ; 현재 플레이어 컨트롤러의 MoveDirection이 1일 경우 send -1
    (if (== (`self.Player_MoveDirection`) 1)
      (`GridManager.AdvanceAllUnits` _gridmanager -1)
      (else
        (`GridManager.AdvanceAllUnits` _gridmanager 1)))
    ; 현재 턴수 증가
    (bind _output_get (set `/Game/CoreClave/Assets/GameModeFiles/GS_CoreClave.CurrentTurn` (+ (`/Game/CoreClave/Assets/GameModeFiles/GS_CoreClave.CurrentTurn` _as_gs_core_clave) 1) _as_gs_core_clave))
    (`KismetSystemLibrary.PrintString` (`KismetTextLibrary.Conv_TextToString` (`|FormatText` "현재턴수{0}" _output_get)))
    (set `/Game/CoreClave/Assets/GameModeFiles/PS_CoreClave.bHasPassButton` true (`self.As PS Core Clave`))))

(event `Server_SpawnUnit`
  (params (SpawnLocation :type "Vector Structure") (Col :type Integer) (Row :type Integer) (CardId :type Name))
  (bind _gridmanager (`self.GridManager`))
  (bind _player_movedirection (`self.Player_MoveDirection`))
  ; 로컬 컨트롤러 플레이어의 인덱스를 기반으로 스폰하고자 하는 유닛을 스 폰
  (`KismetSystemLibrary.PrintString` (`KismetStringLibrary.Conv_IntToString` Col))
  (`KismetSystemLibrary.PrintString` (`KismetStringLibrary.Conv_IntToString` Row))
  (`KismetSystemLibrary.PrintString` "스폰 호출됨")
  (switch `int` (`self.MyPlayer_idx`)
    (:`0`
      (bind _returnvalue (`GridManager.SpawnUnitAtCell` _gridmanager Row Col "/Game/CoreClave/Assets/Card_normal_0.Card_normal_0_C"))
      (if (`KismetSystemLibrary.IsValid` _returnvalue)
        (`self.K2_SetActorRotation` _returnvalue (struct :`Yaw` -90.0) false)
        (bind _ascard_unit_actor (cast `CardUnitActor` _returnvalue))
        (set `CardUnitActor.MoveDirection` _player_movedirection _ascard_unit_actor)
        (`CardUnitActor.InitializeUnit` _ascard_unit_actor CardId)
        (`KismetSystemLibrary.PrintString` "0번 인덱스 플레이어 병사 스폰!")))
    (:`1`
      (bind _returnvalue_2 (`GridManager.SpawnUnitAtCell` _gridmanager Row Col "/Game/CoreClave/Assets/Card_normal_0.Card_normal_0_C"))
      (if (`KismetSystemLibrary.IsValid` _returnvalue_2)
        (`self.K2_SetActorRotation` _returnvalue_2 (struct :`Yaw` 90.0) false)
        (bind _ascard_unit_actor_2 (cast `CardUnitActor` _returnvalue_2))
        (set `CardUnitActor.MoveDirection` _player_movedirection _ascard_unit_actor_2)
        (`CardUnitActor.InitializeUnit` _ascard_unit_actor_2 CardId)
        (`KismetSystemLibrary.PrintString` "1번 인덱스 플레이어 병사 스폰!")))))

(event `ReRoll`
  ; 서버(GM)에서 AP 포인트 변경하도록 호출
  (`/Game/CoreClave/Assets/GameModeFiles/GM_CoreClave.Server_Reroll` (`self.As GM Core Clave`) self))

(fn `OnRep_MyPlayer_idx`
  (`self.SetupCamera`)
  (`KismetSystemLibrary.PrintString` "OnRep 실행됨"))

(fn `OnRep_Player State`
  (bind _mycardui (`self.MyCardUI`))
  (`/Engine/EditorBlueprintResources/StandardMacros.IsValid` (`self.Player State`)
    (:`Is Valid`
      (`/Engine/EditorBlueprintResources/StandardMacros.IsValid` _mycardui
        (:`Is Valid`
          (`/Game/CoreClave/Assets/UI/CardUI.Initialize PS&Mana` _mycardui self)
          (return))))))

(fn `SetupCamera`
  (if (`self.IsLocalController`)
    (switch `int` (`self.MyPlayer_idx`)
      (:`0`
        (bind _outactors (`GameplayStatics.GetAllActorsOfClassWithTag` "/Script/Engine.CameraActor" "Player1"))
        (set `self.Camaer(Player1)` _outactors)
        (`self.SetViewTargetWithBlend` self (`|GetArrayItem` _outactors) 0.0 "VTBlend_Linear" 20.0 false))
      (:`1`
        (bind _outactors_2 (`GameplayStatics.GetAllActorsOfClassWithTag` "/Script/Engine.CameraActor" "Player2"))
        (set `self.Camera(Player2)` _outactors_2)
        (`self.SetViewTargetWithBlend` self (`|GetArrayItem` _outactors_2) 0.0 "VTBlend_Linear" 20.0 false)))
    (bind _returnvalue (`|CreateWidget` "/Game/CoreClave/Assets/UI/CardUI.CardUI_C" self))
    (bind _output_get (set `self.MyCardUI` _returnvalue))
    (`UserWidget.AddToViewport` _output_get 0)
    (`WidgetBlueprintLibrary.SetInputMode_GameAndUIEx` self _returnvalue "DoNotLock" false)
    (else
      (`KismetSystemLibrary.PrintString` "로컬 플레이어 아님!"))))

(fn `UserConstructionScript`)